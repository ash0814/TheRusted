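; BP_DoorOpen is an overlap-triggered actor that opens the store door, raising it and marking the store open.
; On any actor overlap, it checks BP_TheRustedGameModeBase that the store is closed and can open.
; It then plays the DoorOpen timeline on the first StaticMeshActor tagged "OpenDoor", adding a lerped Z offset to its current location each update, so movement accumulates.
; When the timeline finishes, it sets IsStoreOpen on the game mode.
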(event EventBeginPlay)

(event EventTick
  (params (DeltaSeconds :type Float%20%28single-precision%29)))

(event Collision|EventActorBeginOverlap
  (params (OtherActor :type Actor%20Object%20Reference))
  (bind _returnvalue (Game|GetGameMode))
  (bind _asbp_the_rusted_game_mode_base (Utilities|Casting|CastToBP_TheRustedGameModeBase _returnvalue))
  (bind _returnvalue_2 (Class|TheRustedGameModeBase|GetIsStoreOpen _asbp_the_rusted_game_mode_base))
  (if (not _returnvalue_2)
    (bind _returnvalue_3 (Class|TheRustedGameModeBase|GetCanStoreOpen _asbp_the_rusted_game_mode_base))
    (if _returnvalue_3
      (bind _outactors (Actor|GetAllActorsOfClasswithTag "/Script/Engine.StaticMeshActor" "OpenDoor"))
      (bind _newtrack_0 (Timeline|DoorOpen Play)
        (:Update
          (Transformation|SetActorLocation (Utilities|Array|Get(acopy) _outactors) (+ (Transformation|GetActorLocation (Utilities|Array|Get(acopy) _outactors)) (Math|Vector|MakeVector 0.0 0.0 (Math|Float|Lerp 0.0 1e+01 _newtrack_0))) false false))
        (:Finished
          (Class|TheRustedGameModeBase|SetIsStoreOpen _asbp_the_rusted_game_mode_base true))))))

(fn ConstructionScript)