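; Healer enemy character Blueprint that supplies attack, patrol, sensing and movement-speed functions.
; Attack only plays a shotgun ironsights fire montage on the mesh, with no damage or healing logic in this file.
; GetPatrolSpline returns its BPSpline, and SetMovementSpeed maps idle, walk and sprint states to the movement component's max walk speed.
; CanSenseActor is a stub that always returns false.
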(event Custom|Attack
  (Animation|Montage|PlayMontage (Variables|Character|GetMesh) "/Game/Enemy/Healer/Animation/MT_Healer_Fire_Shotgun_Ironsights_Montage.MT_Healer_Fire_Shotgun_Ironsights_Montage"))

(event EventBeginPlay)

(fn ConstructionScript)

(fn CanSenseActor
  (params (Actor :type Float%20%28double-precision%29) (Sense :type E_HealerAISense%20Enum :default "NewEnumerator0"))
  (return false))

(fn GetPatrolSpline
  (return (Variables|Default|GetBP_Spline)))

(fn SetMovementSpeed
  (params (Speed :type E_HealerMovementSpeed%20Enum :default "NewEnumerator0"))
  (bind _output_get (Variables|/Script/Engine.CharacterMovementComponent|SetMaxWalkSpeed (Variables|Character|GetCharacterMovement) (Utilities|Select :Index Speed :NewEnumerator0 0.0 :NewEnumerator1 3e+02 :NewEnumerator2 5e+02)))
  (return _output_get))