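; Gatekeeper enemy character Blueprint that exposes patrol, movement speed, attack and death hooks, with state handled by its AI controller.
; It returns its patrol spline and maps an idle, walk or sprint setting to the character's max walk speed.
; Attack plays a rifle ironsights fire montage with only a debug print on completion, and death tells AIC_Enemy_Gatekeeper to enter its dead state.
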(event EventBeginPlay)

(event Collision|EventActorBeginOverlap
  (params (OtherActor :type Actor%20Object%20Reference)))

(event EventTick
  (params (DeltaSeconds :type Float%20%28single-precision%29)))

(event EventOnDieSetState
  (bind _asaic_enemy_gatekeeper (Utilities|Casting|CastToAIC_Enemy_Gatekeeper (AI|GetAIController self)))
  (Default|SetStateDead _asaic_enemy_gatekeeper))

(event EventAttack
  (Animation|Montage|PlayMontage (Variables|Character|GetMesh) "/Game/Enemy/Gatekeeper/Animation/Fire_Rifle_Ironsights_Montage.Fire_Rifle_Ironsights_Montage"
    (:OnCompleted
      (Development|PrintString "Hello"))))

(fn ConstructionScript)

(fn GetPatrolSpline
  (return (Variables|Default|GetPatrolSpline)))

(fn SetMovementSpeed
  (params (Speed :type E_EnemyMovementSpeedType%20Enum :default "NewEnumerator0"))
  (bind _output_get (Variables|/Script/Engine.CharacterMovementComponent|SetMaxWalkSpeed (Variables|Character|GetCharacterMovement) (Utilities|Select :Index Speed :NewEnumerator0 0.0 :NewEnumerator1 2e+02 :NewEnumerator2 5e+02)))
  (return _output_get))