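; BP_PatrolSpline is an enemy patrol route actor for the Shooter enemy, built on a spline.
; It tracks a current point index, which ChangeIdx steps one point forward or backward at random, wrapping around at either end so the route acts as a loop.
; GetSplinePointLocation returns the world location of the current point.
; The actor moves nothing itself and runs no active logic on BeginPlay or Tick.
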(event Custom|Change%20Idx
  (bind _patrol_spline (Variables|Default|GetPatrol%20Spline))
  (bind _returnvalue (Spline|GetNumberOfSplinePoints _patrol_spline))
  (Variables|Default|SetMove%20Dir (- (* (Math|Random|RandomIntegerinRange 0 1) 2) 1))
  (if (> (+ (Variables|Default|GetSpline%20Idx) (Variables|Default|GetMove%20Dir)) (- _returnvalue 1))
    (Variables|Default|SetSpline%20Idx (- (+ (Variables|Default|GetSpline%20Idx) (Variables|Default|GetMove%20Dir)) _returnvalue))
    (elif (< (+ (Variables|Default|GetSpline%20Idx) (Variables|Default|GetMove%20Dir)) 0)
      (Variables|Default|SetSpline%20Idx (+ (+ (Variables|Default|GetSpline%20Idx) (Variables|Default|GetMove%20Dir)) _returnvalue))
      (else
        (Variables|Default|SetSpline%20Idx (+ (Variables|Default|GetSpline%20Idx) (Variables|Default|GetMove%20Dir)))))))

(event EventBeginPlay)

(event Collision|EventActorBeginOverlap
  (params (OtherActor :type Actor%20Object%20Reference)))

(event EventTick
  (params (DeltaSeconds :type Float%20%28single-precision%29)))

(fn ConstructionScript)

(fn GetSplinePointLocation
  (return (Spline|GetLocationatSplinePoint (Variables|Default|GetPatrol%20Spline) (Variables|Default|GetSpline%20Idx) "World")))